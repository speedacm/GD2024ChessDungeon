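; BP_Grid is an actor that builds a tile grid from its size, count and shape settings at its location.
; The construction script calls SpawnGrid, which clears old instances and takes mesh, material and mesh size from the shape's row in DT_GridShapeData.
; It snaps the center to tile size, derives the bottom-left corner with even/odd count correction, then adds scaled tiles to one InstancedStaticMesh.
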(fn `CalcCenterandBottomLeft`
  (returns (BottomLeft :type "Vector Structure") (Center :type "Vector Structure"))
  (locals (C :type "Vector Structure" :default (0.0 0.0 0.0)))
  (bind (_gridtilecount_x _gridtilecount_y) (`KismetMathLibrary.BreakVector2D` (`self.GridTileCount`)))
  (set `local.C` (`/Game/Dynamic/Blueprints/Core/Utilities/BFL_Utilities.Snap Vector to Vector` (`self.GridCenterLocation`) (`self.GridTileSize`)))
  (return (- (- (`local.C`) (* (/ (- (`self.GridTileCount`) (`KismetMathLibrary.MakeVector2D` (`KismetMathLibrary.SelectFloat` 0.0 1.0 (`/Game/Dynamic/Blueprints/Core/Utilities/BFL_Utilities.Is Float Even` _gridtilecount_x)) (`KismetMathLibrary.SelectFloat` 0.0 1.0 (`/Game/Dynamic/Blueprints/Core/Utilities/BFL_Utilities.Is Float Even` _gridtilecount_y)))) 2.0) (`self.GridTileSize`))) (0.0 0.0 0.0)) (`local.C`)))

(fn `DestroyGrid`
  (`InstancedStaticMeshComponent.ClearInstances` (`self.InstancedStaticMesh`)))

(fn `Get Current Shape Data`
  (returns (ReturnValue :type "/Game/Dynamic/Blueprints/Core/Grid/S_GridShapeData Structure"))
  (bind _returnvalue (`|GetEnumeratorNameAsString` (`self.GridTileShape`)))
  (bind _returnvalue_2 (`|GetDataTableRow` "/Game/Dynamic/Blueprints/Core/Grid/DT_GridShapeData.DT_GridShapeData" (`KismetStringLibrary.Conv_StringToName` _returnvalue))
    (:`then`
      _)
    (:`RowNotFound`
      (`KismetSystemLibrary.PrintString` (`KismetStringLibrary.Concat_StrStr` _returnvalue) true true (struct :`R` 1.0 :`G` 0.031819 :`A` 1.0) 5.0)))
  (return _returnvalue_2))

(fn `Spawn Grid`
  (params (CenterLocation :type "Vector Structure") (TileSize :type "Vector Structure") (TileCount :type "Vector2D Structure") (Shape :type "/Game/Dynamic/Blueprints/Core/Grid/E_GridShape Enum" :default "NewEnumerator0"))
  (locals (X :type Integer) (y :type Integer) (TileTransform :type "Transform Structure"))
  (bind _instancedstaticmesh (`self.InstancedStaticMesh`))
  (bind (_tilecount_x _tilecount_y) (`KismetMathLibrary.BreakVector2D` (`local.TileCount`)))
  (bind (_gridtilecount_x _gridtilecount_y) (`KismetMathLibrary.BreakVector2D` (`self.GridTileCount`)))
  (bind _gridtilecount_x_2 (`KismetMathLibrary.BreakVector2D` (`self.GridTileCount`)))
  (bind (_meshsize _mesh _meshmaterial _flatmesh _flatfilledmaterial _flatbordermaterial) (break `/Game/Dynamic/Blueprints/Core/Grid/S_GridShapeData` (`self.Get Current Shape Data`)))
  ;[1 1 1] Set Variables
  (set `self.GridCenterLocation` CenterLocation)
  (set `self.GridTileSize` TileSize)
  (set `self.GridTileShape` Shape)
  (set `self.GridTileCount` (`KismetMathLibrary.MakeVector2D` (`KismetMathLibrary.Conv_IntToDouble` (`KismetMathLibrary.Round` _tilecount_x)) (`KismetMathLibrary.Conv_IntToDouble` (`KismetMathLibrary.Round` _tilecount_y))))
  (`self.DestroyGrid`)
  (`StaticMeshComponent.SetStaticMesh` _instancedstaticmesh _mesh)
  (`PrimitiveComponent.SetMaterial` _instancedstaticmesh 0 _flatbordermaterial)
  ;[1 1 1] Ugly ah find bottom left corner of the grid and start spawning tiles there
  (bind (_bottomleft _center) (`self.CalcCenterandBottomLeft`))
  (set `self.GridBottomLeftCornerLocation` _bottomleft)
  (set `self.GridCenterLocation` _center)
  (for _index (range (`KismetMathLibrary.Round` _gridtilecount_x_2))
    (set `local.X` _index)
    (for _index_2 (range (`KismetMathLibrary.Round` _gridtilecount_y))
      (set `local.y` _index_2)
      (set `local.TileTransform` (`KismetMathLibrary.MakeTransform` (+ (`self.GridBottomLeftCornerLocation`) (* (`self.GridTileSize`) (`KismetMathLibrary.MakeVector` (`KismetMathLibrary.Conv_IntToDouble` (`local.X`)) (`KismetMathLibrary.Conv_IntToDouble` (`local.y`))))) (struct) (/ (`self.GridTileSize`) (`.MeshSize_2_D78069EF4586FA476E78749660218D57` (break `/Game/Dynamic/Blueprints/Core/Grid/S_GridShapeData` (`self.Get Current Shape Data`))))))
      (`InstancedStaticMeshComponent.AddInstance` (`self.InstancedStaticMesh`) (`local.TileTransform`) true))))

(fn `UserConstructionScript`
  (`self.Spawn Grid` (`self.K2_GetActorLocation`) (`self.GridTileSize`) (`self.GridTileCount`) (`self.GridTileShape`)))